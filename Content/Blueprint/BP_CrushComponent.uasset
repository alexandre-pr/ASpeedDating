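; Character component for a speed-dating game that handles crushes between players and keeps a love score for each partner.
; On the server, it reports CrushCollision overlaps to the GameMode's crush manager by player IDs, and waits tick by tick for PlayerState before binding dialogue-start.
; When a dialogue ends with matching valid answers, it increments that partner's LoveMeter and passes the score to UpdateLoveMeter.
; Both OnRep functions are empty.
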(event Custom|HandleBeginOverlap
  (params (OverlappedComponent :type Primitive%20Component%20Object%20Reference) (OtherActor :type Actor%20Object%20Reference) (OtherComp :type Primitive%20Component%20Object%20Reference) (OtherBodyIndex :type Integer) (bFromSweep :type Boolean) (SweepResult :type Hit%20Result%20Structure%20%28by%20ref%29))
  (if (not (== OtherActor (Components|GetOwner)))
    (bind _asbp_aspeed_dating_character (Utilities|Casting|CastToBP_ASpeedDatingCharacter OtherActor))
    (CallFunction|OnCrush (PlayerState|GetUniqueID (Variables|/Script/Engine.Pawn|GetPlayerState (Variables|Default|GetOwner))) (PlayerState|GetUniqueID (Variables|/Script/Engine.Pawn|GetPlayerState _asbp_aspeed_dating_character)))))

(event Custom|OnCrush
  (params (This :type Unique%20Net%20Id%20Repl%20Structure) (Other :type Unique%20Net%20Id%20Repl%20Structure))
  ;[1 1 1] Tell the server that a collision happened
  (bind _asbp_game_mode (Utilities|Casting|CastToBP_GameMode (Game|GetGameMode)))
  (Default|OnCrush (Variables|/Game/GameFrameWork/BP_GameMode.BP_GameMode_C|GetBP_CrushManager _asbp_game_mode) This Other))

(event Custom|HandleCrushDialogueInit
  (params (CrushInstance :type BP%20Crush%20Instance%20Object%20Reference))
  (bind _player1 (Variables|/Game/Blueprint/BP_CrushInstance.BP_CrushInstance_C|GetPlayer1 CrushInstance))
  ;[1 1 1] On Server
  (Variables|Server|SetCrushInstance CrushInstance)
  (Variables|Server|SetOtherPlayer (select (== (Game|GetPlayerStatefromUniqueNetId _player1) (Variables|/Script/Engine.Pawn|GetPlayerState (Variables|Default|GetOwner))) (Variables|/Game/Blueprint/BP_CrushInstance.BP_CrushInstance_C|GetPlayer2 CrushInstance) _player1))
  (EventDispatchers|BindEventtoInstanceonCrushDialogueEnd (Variables|Server|GetCrushInstance) (EventDispatchers|CreateEvent :!event Custom|HandleCrushEnd))
  (Development|PrintString "InitilaizedCrushServer"))

(event Custom|HandleCrushEnd
  (params (CrushInstance :type BP%20Crush%20Instance%20Object%20Reference))
  (bind _player1answer (Variables|/Game/Blueprint/BP_CrushInstance.BP_CrushInstance_C|GetPlayer1Answer CrushInstance))
  (bind _otherplayer (Variables|Server|GetOtherPlayer))
  (bind _lovemeter (Variables|Server|GetLoveMeter))
  (bind (_value _returnvalue) (Utilities|Map|Find _lovemeter _otherplayer))
  ;[1 1 1] On Server
  (if (and (== _player1answer (Variables|/Game/Blueprint/BP_CrushInstance.BP_CrushInstance_C|GetPlayer2Answer CrushInstance)) (!= _player1answer -1))
    (Development|PrintString "Crush Answer Success")
    (Utilities|FlowControl|Sequence
      (:then_0
        (if _returnvalue
          (Variables|Default|SetNewLoveMeterScore (+ _value 1))
          (else
            (Variables|Default|SetNewLoveMeterScore 1))))
      (:then_1
        (Utilities|Map|Add (Variables|Server|GetLoveMeter) (Variables|Server|GetOtherPlayer) (Variables|Default|GetNewLoveMeterScore))
        (CallFunction|UpdateLoveMeter (Variables|Default|GetNewLoveMeterScore) (Variables|Server|GetOtherPlayer))
        (Development|PrintString "CalledForLoveReplication")))))

(event Custom|UpdateLoveMeter
  (params (NewLoveMeterScore :type Integer) (OtherPlayer :type Unique%20Net%20Id%20Repl%20Structure))
  (Utilities|Map|Add (Variables|Server|GetLoveMeter) OtherPlayer NewLoveMeterScore)
  (Development|PrintString (Utilities|String|Append "LoveMeter: " (Utilities|String|ToString(Integer) NewLoveMeterScore))))

(event EventBeginPlay
  (bind _asbp_aspeed_dating_character (Utilities|Casting|CastToBP_ASpeedDatingCharacter (Components|GetOwner)))
  (Variables|Default|SetOwner _asbp_aspeed_dating_character)
  (Utilities|FlowControl|Sequence
    (:then_0
      ;[1 1 1] OnServer
      (if (Networking|IsServer)
        (Variables|Default|SetCrushState "NewEnumerator1")
        (Collision|BindEventtoOnComponentBeginOverlap (Variables|/Game/GameFrameWork/BP_ASpeedDatingCharacter.BP_ASpeedDatingCharacter_C|GetCrushCollision (Variables|Default|GetOwner)) (EventDispatchers|CreateEvent :!event Custom|HandleBeginOverlap))
        (if (Utilities|IsValid (Variables|/Script/Engine.Pawn|GetPlayerState (Variables|Default|GetOwner))) :!label _label
          (bind _asbp_aspeed_dating_player_state (Utilities|Casting|CastToBP_AspeedDatingPlayerState (Variables|/Script/Engine.Pawn|GetPlayerState (Variables|Default|GetOwner))))
          (EventDispatchers|BindEventtoOnCrushDialogueInit _asbp_aspeed_dating_player_state (EventDispatchers|CreateEvent :!event Custom|HandleCrushDialogueInit))
          (Development|PrintString "CrushComponetn Initalized On Server")
          (else
            (Utilities|FlowControl|DelayUntilNextTick)
            (goto _label)))))))

(event EventTick
  (params (DeltaSeconds :type Float%20%28single-precision%29)))

(fn OnRepCrushState)

(fn OnRepLocalLoveScore)
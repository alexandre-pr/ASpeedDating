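; BP_AvatarBase is a base avatar with a customizable mesh, body color and eye style.
; The construction script creates dynamic material instances for the body and both eyes, then applies the stored color and eye type.
; SetColor maps preset colors to a material parameter, while SetEye sets paired open and closed eye textures on both eyes.
; UpdateAvatar swaps the body mesh and relative transform from the Avatars collection by ID.
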(event Custom|SetColor
  (params (NewParam :type EAvatarColor%20Enum :default "NewEnumerator0"))
  (bind _output_get (Variables|Default|SetColor NewParam))
  (Rendering|Material|SetVectorParameterValue (Variables|Default|GetMID) "Color" (Utilities|Select :Index _output_get :NewEnumerator0 "(R=0.066626,G=0.184475,B=1.000000,A=1.000000)" :NewEnumerator1 "(R=0.791298,G=0.003347,B=0.000000,A=1.000000)" :NewEnumerator2 "(R=1.000000,G=0.318547,B=0.000000,A=1.000000)" :NewEnumerator3 "(R=0.822786,G=0.039546,B=0.266356,A=1.000000)" :NewEnumerator4 "(R=0.270498,G=0.417885,B=0.147027,A=1.000000)" :NewEnumerator5 "(R=1.000000,G=1.000000,B=1.000000,A=1.000000)") :!class /Script/Engine.MaterialInstanceDynamic))

(event Custom|SetEye
  (params (NewParam :type Integer))
  (Variables|Default|SetEyeType NewParam)
  (Rendering|Material|SetTextureParameterValue (Variables|Default|GetMIDLeft) "OpenEye" (Utilities|Select :Index (Variables|Default|GetEyeType) :Option%200 "/Game/Assets/Textures/Eyes/1A.1A" :Option%201 "/Game/Assets/Textures/Eyes/2A.2A" :Option%202 "/Game/Assets/Textures/Eyes/3A.3A" :Option%203 "/Game/Assets/Textures/Eyes/4A.4A" :Option%204 "/Game/Assets/Textures/Eyes/5A.5A" :Option%205 "/Game/Assets/Textures/Eyes/6A.6A" :Option%206 "/Game/Assets/Textures/Eyes/7A.7A" :Option%207 "/Game/Assets/Textures/Eyes/8A.8A"))
  (Rendering|Material|SetTextureParameterValue (Variables|Default|GetMIDLeft) "CloseEye" (Utilities|Select :Index (Variables|Default|GetEyeType) :Option%200 "/Game/Assets/Textures/Eyes/1B.1B" :Option%201 "/Game/Assets/Textures/Eyes/2B.2B" :Option%202 "/Game/Assets/Textures/Eyes/3B.3B" :Option%203 "/Game/Assets/Textures/Eyes/4B.4B" :Option%204 "/Game/Assets/Textures/Eyes/5B.5B" :Option%205 "/Game/Assets/Textures/Eyes/6B.6B" :Option%206 "/Game/Assets/Textures/Eyes/7B.7B" :Option%207 "/Game/Assets/Textures/Eyes/8B.8B")))

(event EventBeginPlay)

(event Collision|EventActorBeginOverlap
  (params (OtherActor :type Actor%20Object%20Reference)))

(event EventTick
  (params (DeltaSeconds :type Float%20%28single-precision%29)))

(fn ConstructionScript
  (bind _staticmesh (Variables|Default|GetStaticMesh))
  (bind _eyeleft (Variables|Default|GetEyeLeft))
  (bind _eyeright (Variables|Default|GetEyeRight))
  (bind _returnvalue (Rendering|Material|CreateDynamicMaterialInstance _staticmesh 0 (Rendering|Material|GetMaterial _staticmesh 0) "None" :!class /Script/Engine.PrimitiveComponent))
  (Variables|Default|SetMID _returnvalue)
  (CallFunction|SetColor (Variables|Default|GetColor))
  (bind _returnvalue_2 (Rendering|Material|CreateDynamicMaterialInstance _eyeright 0 (Rendering|Material|GetMaterial _eyeright 0) "None" :!class /Script/Engine.PrimitiveComponent))
  (Variables|Default|SetMIDRight _returnvalue_2)
  (bind _returnvalue_3 (Rendering|Material|CreateDynamicMaterialInstance _eyeleft 0 (Rendering|Material|GetMaterial _eyeleft 0) "None" :!class /Script/Engine.PrimitiveComponent))
  (Variables|Default|SetMIDLeft _returnvalue_3)
  (CallFunction|SetEye (Variables|Default|GetEyeType)))

(fn UpdateAvatar
  (params (ID :type Integer))
  (Variables|Default|SetChosenAvatar ID)
  (Transformation|SetRelativeTransform (Variables|Default|GetStaticMesh) (.maintransform (Utilities|Array|Get(acopy) (Variables|Default|GetAvatars) (Variables|Default|GetChosenAvatar))) false false)
  (Components|StaticMesh|SetStaticMesh (Variables|Default|GetStaticMesh) (.mainmesh (Utilities|Array|Get(acopy) (Variables|Default|GetAvatars) (Variables|Default|GetChosenAvatar)))))
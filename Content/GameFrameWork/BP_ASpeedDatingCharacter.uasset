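; Player character Blueprint for a speed dating game, with a randomly chosen, colored avatar and a love meter widget hidden for its local player.
; The server picks the replicated model and color; BeginPlay and OnRep spawn the avatar onto a Scene component.
; BeginPlay also teleports to a random navigable point and retries each tick until PlayerState is valid to create the widget.
; Tick sways the avatar sideways with a velocity-scaled cosine.
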(event Custom|ChooseModelReplication
  (params (ChosenModel :type F%20Avatar%20Type%20Structure))
  (bind _returnvalue (Game|SpawnActorfromClass (Utilities|Array|Get(acopy) (Variables|Default|GetAvatars) (.modelnum ChosenModel)) (Math|Transform|MakeTransform "0, 0, 0" "0, 0, 0" "1.000000,1.000000,1.000000") "Undefined" 0 0))
  (Transformation|AttachComponentToComponent _returnvalue (Variables|Default|GetScene) "None" "SnapToTarget" "SnapToTarget" "SnapToTarget" true)
  (bind _output_get (Variables|Default|SetSpawnedAvatar _returnvalue))
  (Default|SetColor _output_get (.color ChosenModel)))

(event EventBeginPlay
  (bind _playerstate (Variables|GetPlayerState))
  (CallFunction|ChoseModel)
  (CallFunction|ChooseModelReplication (Variables|Default|GetModelNumber))
  (CallFunction|SpawnRandom)
  (Development|SetHiddeninGame (Variables|Default|GetWidget) (Pawn|IsLocallyControlled) false)
  (Utilities|IsValid _playerstate :!label _label
    (:Is%20Valid
      (bind _returnvalue (UserInterface|CreateWidget "/Game/Assets/UI/UW_LoveMeter.UW_LoveMeter_C" 0 (PlayerState|GetUniqueID _playerstate)))
      (UserInterface|SetWidget (Variables|Default|GetWidget) _returnvalue)
      (Development|PrintString "LoveMeterInitialized"))
    (:Is%20Not%20Valid
      (Utilities|FlowControl|DelayUntilNextTick)
      (goto _label))))

(event Collision|EventActorBeginOverlap
  (params (OtherActor :type Actor%20Object%20Reference)))

(event EventTick
  (params (DeltaSeconds :type Float%20%28single-precision%29))
  (bind _scene (Variables|Default|GetScene))
  (bind _relativelocation (Variables|/Script/Engine.SceneComponent|GetRelativeLocation _scene))
  (Variables|Default|SetAnimationTimer (+ (Variables|Default|GetAnimationTimer) (* (Utilities|Time|GetWorldDeltaSeconds) (Variables|Default|GetAnimationSpeed) (Math|Vector|VectorLength (Variables|/Script/Engine.MovementComponent|GetVelocity (Variables|Character|GetCharacterMovement))))))
  (Transformation|SetRelativeLocation _scene (Math|Vector|MakeVector (.x _relativelocation) (* (Math|Trig|Cos(Degrees) (Variables|Default|GetAnimationTimer)) (Variables|Default|GetAnimationRange) (Math|Vector|VectorLength (Variables|/Script/Engine.MovementComponent|GetVelocity (Variables|Character|GetCharacterMovement)))) (.z _relativelocation)) false false))

(event Collision|EventHit
  (params (MyComp :type Primitive%20Component%20Object%20Reference) (Other :type Actor%20Object%20Reference) (OtherComp :type Primitive%20Component%20Object%20Reference) (bSelfMoved :type Boolean) (HitLocation :type Vector :default "0, 0, 0") (HitNormal :type Vector :default "0, 0, 0") (NormalImpulse :type Vector :default "0, 0, 0") (Hit :type Hit%20Result%20Structure%20%28by%20ref%29)))

(fn ConstructionScript)

(fn SpawnRandom
  (bind _randomlocation (Class|NavigationSystemV1|GetRandomLocationinNavigableRadius (Math|Vector|MakeVector 1.44e+03 1.62e+03 0.0) 1e+03 0 0))
  (Transformation|SetActorLocation _randomlocation false true)
  (Development|PrintString "Hello" true true "(R=1.000000,G=0.000000,B=0.116213,A=1.000000)"))

(fn ChoseModel
  (if (Networking|IsServer)
    (Development|PrintString "Model Chosing")
    (Variables|Default|SetModelNumber (Utilities|Struct|MakeFAvatarType (Math|Random|RandomInteger (Utilities|Array|Length (Variables|Default|GetAvatars))) (Utilities|Enum|ByteToEnumEAvatarColor (Math|Conversions|ToByte(Integer) (Math|Random|RandomInteger (|GetNumEnumEntries))))))))

(fn OnRepModelNumber
  (CallFunction|ChooseModelReplication (Variables|Default|GetModelNumber)))

(fn OnRepModelColor)
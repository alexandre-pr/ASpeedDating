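; HUD for the speed-dating game that shows and removes the crush dialogue panel.
; On BeginPlay it retries each tick until the owning player's PlayerState is valid, then binds to that state's crush dialogue init event.
; Each init creates a UW_CrushPanel for the crush instance, adds it to the viewport and binds the instance's dialogue-end event, which removes the panel.
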(event Custom|HandleCrushDialogueEnd
  (params (CrushInstance :type BP%20Crush%20Instance%20Object%20Reference) (bSuccess :type Boolean) (bDating :type Boolean))
  (Widget|RemovefromParent (Variables|Default|GetCrushPanel)))

(event Custom|HandleCrushDialogueInit
  (params (CrushInstance :type BP%20Crush%20Instance%20Object%20Reference))
  (EventDispatchers|BindEventtoInstanceonCrushDialogueEnd CrushInstance (delegate Custom|HandleCrushDialogueEnd))
  (Development|PrintString "HUDInitCrushDialogue" true true "(R=0.000000,G=0.660000,B=1.000000,A=1.000000)" 1e+01)
  (bind _returnvalue (UserInterface|CreateWidget "/Game/Assets/UI/UW_CrushPanel.UW_CrushPanel_C" (Game|Player|GetOwningPlayerController) CrushInstance))
  (UserInterface|Viewport|AddtoViewport _returnvalue 0)
  (Variables|Default|SetCrushPanel _returnvalue)
  (Development|PrintString "HUDCrushStart" true true "(R=0.000000,G=0.660000,B=1.000000,A=1.000000)" 1e+01))

(event Custom|HandleStartCrushDialogue)

(event Custom|Init)

(event EventBeginPlay
  (if (Utilities|IsValid (Variables|/Script/Engine.Controller|GetPlayerState (Variables|Default|GetPlayerOwner))) :!label _label
    (Development|PrintString "HUDStartInit")
    (bind _asbp_aspeed_dating_player_state (Utilities|Casting|CastToBP_AspeedDatingPlayerState (Variables|/Script/Engine.Controller|GetPlayerState (Game|Player|GetOwningPlayerController))))
    (EventDispatchers|BindEventtoOnCrushDialogueInit _asbp_aspeed_dating_player_state (delegate Custom|HandleCrushDialogueInit))
    (Development|PrintString "HookedOnPS")
    (else
      (Utilities|FlowControl|DelayUntilNextTick)
      (goto _label))))

(event Collision|EventActorBeginOverlap
  (params (OtherActor :type Actor%20Object%20Reference)))

(event EventTick
  (params (DeltaSeconds :type Float%20%28single-precision%29)))

(fn ConstructionScript)
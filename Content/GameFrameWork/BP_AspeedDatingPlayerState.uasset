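; Player state for a speed dating game that relays crush dialogue starts to the players involved.
; On BeginPlay it binds to the game state's crush dialogue event, then after a short delay initializes the speed dating HUD through its player controller, if valid.
; When the event's two player IDs include this state, it rebroadcasts the crush instance through its own dispatcher, with debug prints.
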(event Custom|HandleOnCrushDialogueInit
  (params (Player1 :type Unique%20Net%20Id%20Repl%20Structure) (Player2 :type Unique%20Net%20Id%20Repl%20Structure) (CrushInstance :type BP%20Crush%20Instance%20Object%20Reference))
  (if (or (== (Game|GetPlayerStatefromUniqueNetId Player1) self) (== (Game|GetPlayerStatefromUniqueNetId Player2) self))
    (Default|CallOnCrushDialogueInit CrushInstance)
    (Development|PrintString "CrushDialogueInitPlayerState" true true "(R=0.000000,G=0.660000,B=1.000000,A=1.000000)" 1e+01)))

(event EventBeginPlay
  (bind _self self)
  (bind _returnvalue (Game|GetPlayerController _self))
  (Development|PrintString "PSBeginPlay")
  (bind _asbp_game_state (Utilities|Casting|CastToBP_GameState (Game|GetGameState)))
  (EventDispatchers|BindEventtoOnCrushDialogueInit _asbp_game_state (delegate Custom|HandleOnCrushDialogueInit))
  (Utilities|FlowControl|Sequence
    (:then_0
      (Utilities|FlowControl|Delay 2.0)
      (Utilities|IsValid _returnvalue
        (:Is%20Valid
          (bind _asbp_aspeed_dating_hud (Utilities|Casting|CastToBP_AspeedDatingHUD (HUD|GetHUD _returnvalue)))
          (Default|Init _asbp_aspeed_dating_hud))))))

(event EventTick
  (params (DeltaSeconds :type Float%20%28single-precision%29)))

(fn ConstructionScript)